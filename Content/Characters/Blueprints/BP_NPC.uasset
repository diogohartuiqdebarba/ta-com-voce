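; BP_NPC is an AI character for a tag game that switches between chasing and fleeing roles.
; On BeginPlay it binds to the TagSystem's set-It-actor event.
; Whenever It changes, its AI controller runs the It behavior tree if this NPC is It, otherwise the RunAway tree.
; It records which tree was last chosen and prints debug messages.
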(event Custom|ChangeIt
  (params (It :type Actor%20Object%20Reference) (TagFree :type Boolean))
  (CallFunction|ChangeBehaviorTree It))

(event EventBeginPlay
  (Development|PrintString "Start NPC." true true "(R=1.000000,G=0.000000,B=0.068582,A=1.000000)")
  (|CallParentFunction)
  (EventDispatchers|BindEventtoSetItActor (Variables|Default|GetTagSystem) (delegate Custom|ChangeIt)))

(fn ConstructionScript
  (|CallParentFunction))

(fn ChangeBehaviorTree
  (params (It :type Actor%20Object%20Reference%20%28by%20ref%29))
  (bind _self self)
  (bind _returnvalue (AI|GetAIController _self))
  (if (== _self It)
    (AI|RunBehaviorTree _returnvalue "/Game/Characters/AI/AI_BT_It.AI_BT_It")
    (Variables|Default|SetLastBehaviorTree "NewEnumerator0")
    (Development|PrintString "AI: It" true true "(R=1.000000,G=0.833552,B=0.000000,A=1.000000)")
    (else
      (AI|RunBehaviorTree _returnvalue "/Game/Characters/AI/AI_BT_RunAway.AI_BT_RunAway")
      (Variables|Default|SetLastBehaviorTree "NewEnumerator1")
      (Development|PrintString "AI: Run Away"))))