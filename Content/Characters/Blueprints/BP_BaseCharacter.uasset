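; Base player character that selects mirror actors by looking at them and takes part in a game of tag.
; A looping timer traces from the camera, selecting or deselecting actors through SelectActorsInterface and binding their unselect event.
; Left click locks the selected mirror by pausing the trace; right click resumes it.
; Hits between characters pass "It" through BP_TagSystem while TagFree is set, then clear that flag.
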(event Custom|CheckSightLine
  (bind _returnvalue (Game|GetPlayerCameraManager 0))
  (bind _returnvalue_2 (Camera|GetCameraLocation _returnvalue))
  ;[1 0.9473 0.4386] Select Actor System
  (if (Variables|Default|GetNotSelected)
    (bind (_outhit _returnvalue_3) (Collision|LineTraceForObjects _returnvalue_2 (+ _returnvalue_2 (* (Transformation|GetActorForwardVector _returnvalue) "2500.000000,2500.000000,2500.000000")) (Utilities|Array|MakeArray "ObjectTypeQuery2") false 0 "None"))
    (if _returnvalue_3
      (if (Utilities|DoesObjectImplementInterface (.hitactor _outhit) "/Game/MirrorSystem/SelectMirror/SelectActorsInterface.SelectActorsInterface_C")
        (bind _isselected (Class|SelectActorsInterface|IsSelected?(Message) (.hitactor _outhit)))
        (if (not _isselected)
          (Utilities|IsValid (Variables|Default|GetSelectedMirror)
            (:Is%20Valid
              (Class|SelectActorsInterface|DeselectActor(Message) (Variables|Default|GetSelectedMirror)))
            (:Is%20Not%20Valid
              _))
          (Class|SelectActorsInterface|SelectActor(Message) (.hitactor _outhit))
          (bind _output_get (Variables|Default|SetSelectedMirror (.hitactor _outhit)))
          (Default|CallChangeSelectedMirror _output_get)
          (bind _asmirror_instance (Utilities|Casting|CastToMirrorInstance (Variables|Default|GetSelectedMirror)))
          (bind _output_get_2 (Variables|Default|SetAs%20Mirror%20Instance _asmirror_instance))
          (EventDispatchers|BindEventtoUnselectMirror _output_get_2 (delegate Custom|UnSelectCurrentMirror)))
        (else
          (Utilities|IsValid (Variables|Default|GetSelectedMirror) :!label _label
            (:Is%20Valid
              (Class|SelectActorsInterface|DeselectActor(Message) (Variables|Default|GetSelectedMirror))
              (Variables|Default|SetSelectedMirror 0)))))
      (else
        (goto _label)))))

(event Custom|UnSelectCurrentMirror
  ;[1 0.9473 0.4386] Select Actor System
  (Utilities|IsValid (Variables|Default|GetSelectedMirror)
    (:Is%20Valid
      (Class|SelectActorsInterface|DeselectActor(Message) (Variables|Default|GetSelectedMirror))
      (Variables|Default|SetSelectedMirror 0)
      (Variables|Default|SetNotSelected true))))

(event Collision|EventHit
  (params (MyComp :type Primitive%20Component%20Object%20Reference) (Other :type Actor%20Object%20Reference) (OtherComp :type Primitive%20Component%20Object%20Reference) (bSelfMoved :type Boolean) (HitLocation :type Vector :default "0, 0, 0") (HitNormal :type Vector :default "0, 0, 0") (NormalImpulse :type Vector :default "0, 0, 0") (Hit :type Hit%20Result%20Structure%20%28by%20ref%29))
  (bind _tagsystem (Variables|Default|GetTagSystem))
  (bind _tagsystem_2 (Variables|Default|GetTagSystem))
  ;[1 0.007292 0.007292] Tag/Untag
  (Utilities|Casting|CastToBP_BaseCharacter Other)
  (if (Variables|/Game/TagSystem/BP_TagSystem.BP_TagSystem_C|GetTagFree _tagsystem)
    (if (== Other (Variables|/Game/TagSystem/BP_TagSystem.BP_TagSystem_C|GetIt _tagsystem))
      (Default|SetIt _tagsystem_2 (Game|GetPlayerCharacter 0))
      (else
        (Default|SetIt _tagsystem_2 Other)))
    (Variables|/Game/TagSystem/BP_TagSystem.BP_TagSystem_C|SetTagFree _tagsystem_2 false)))

(event EventBeginPlay
  (bind _returnvalue (Game|GetPlayerCameraManager 0))
  (bind _returnvalue_2 (Camera|GetCameraLocation _returnvalue))
  ;[1 0.9473 0.4386] Select Actor System
  (bind _returnvalue_3 (Actor|GetActorOfClass "/Game/TagSystem/BP_TagSystem.BP_TagSystem_C"))
  (Variables|Default|SetTagSystem _returnvalue_3)
  (Development|PrintString "Start Base Character.")
  (Utilities|Time|SetTimerbyEvent (delegate Custom|CheckSightLine) 0.1 true)
  (if (Variables|Default|GetNotSelected)
    (bind (_outhit _returnvalue_4) (Collision|LineTraceForObjects _returnvalue_2 (+ _returnvalue_2 (* (Transformation|GetActorForwardVector _returnvalue) "2500.000000,2500.000000,2500.000000")) (Utilities|Array|MakeArray "ObjectTypeQuery2") false 0 "None"))
    (if _returnvalue_4
      (if (Utilities|DoesObjectImplementInterface (.hitactor _outhit) "/Game/MirrorSystem/SelectMirror/SelectActorsInterface.SelectActorsInterface_C")
        (bind _isselected (Class|SelectActorsInterface|IsSelected?(Message) (.hitactor _outhit)))
        (if (not _isselected)
          (Utilities|IsValid (Variables|Default|GetSelectedMirror)
            (:Is%20Valid
              (Class|SelectActorsInterface|DeselectActor(Message) (Variables|Default|GetSelectedMirror)))
            (:Is%20Not%20Valid
              _))
          (Class|SelectActorsInterface|SelectActor(Message) (.hitactor _outhit))
          (bind _output_get (Variables|Default|SetSelectedMirror (.hitactor _outhit)))
          (Default|CallChangeSelectedMirror _output_get)
          (bind _asmirror_instance (Utilities|Casting|CastToMirrorInstance (Variables|Default|GetSelectedMirror)))
          (bind _output_get_2 (Variables|Default|SetAs%20Mirror%20Instance _asmirror_instance))
          (EventDispatchers|BindEventtoUnselectMirror _output_get_2 (delegate Custom|UnSelectCurrentMirror)))
        (else
          (Utilities|IsValid (Variables|Default|GetSelectedMirror) :!label _label
            (:Is%20Valid
              (Class|SelectActorsInterface|DeselectActor(Message) (Variables|Default|GetSelectedMirror))
              (Variables|Default|SetSelectedMirror 0)))))
      (else
        (goto _label)))))

(event Input|MouseEvents|LeftMouseButton
  (params (Key :type Key%20Structure))
  ;[1 1 1] Select/Unselect Mirror
  (:Pressed
    (Utilities|IsValid (Variables|Default|GetSelectedMirror)
      (:Is%20Valid
        (Variables|Default|SetNotSelected false)))))

(event Input|MouseEvents|RightMouseButton
  (params (Key :type Key%20Structure))
  ;[1 1 1] Select/Unselect Mirror
  (:Pressed
    (Variables|Default|SetNotSelected true)))

(fn ConstructionScript)