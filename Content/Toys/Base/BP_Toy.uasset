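; BP_Toy is a base toy prop that briefly slows any BP_BaseCharacter that hits it, playing a stumble sound.
; On hit, a DoOnce gate lowers the character's walk speed, then restores a fixed speed after a short delay, clears IsSlow and resets.
; The gate resets only on that path, so a non-character or already-slow hit leaves it closed.
; The construction script applies the configurable mesh, physical material and material.
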(event Collision|EventHit
  (params (MyComp :type Primitive%20Component%20Object%20Reference) (Other :type Actor%20Object%20Reference) (OtherComp :type Primitive%20Component%20Object%20Reference) (bSelfMoved :type Boolean) (HitLocation :type Vector :default "0, 0, 0") (HitNormal :type Vector :default "0, 0, 0") (NormalImpulse :type Vector :default "0, 0, 0") (Hit :type Hit%20Result%20Structure%20%28by%20ref%29))
  (Utilities|FlowControl|DoOnce false :!label _label
    (:Completed
      (bind _asbp_base_character (Utilities|Casting|CastToBP_BaseCharacter Other))
      (if (not (Variables|/Game/Characters/Blueprints/BP_BaseCharacter.BP_BaseCharacter_C|GetIsSlow _asbp_base_character))
        (Variables|Default|SetSlowCharacter _asbp_base_character)
        (Variables|/Script/Engine.CharacterMovementComponent|SetMaxWalkSpeed (Variables|/Script/Engine.Character|GetCharacterMovement _asbp_base_character) 3e+02)
        (Audio|PlaySoundatLocation "/Game/Audio/character-stumble-on-toys.character-stumble-on-toys" (Transformation|GetActorLocation _asbp_base_character) "0, 0, 0" 0.48 1.0 0.0 0 0 0 0)
        (Utilities|FlowControl|Delay 0.6)
        (Variables|/Script/Engine.CharacterMovementComponent|SetMaxWalkSpeed (Variables|/Script/Engine.Character|GetCharacterMovement _asbp_base_character) 5e+02)
        (Variables|/Game/Characters/Blueprints/BP_BaseCharacter.BP_BaseCharacter_C|SetIsSlow (Variables|Default|GetSlowCharacter) false)
        (goto _label Reset)))))

(fn ConstructionScript
  (bind _staticmesh (Variables|Default|GetStaticMesh))
  (Components|StaticMesh|SetStaticMesh _staticmesh (Variables|Default|GetMesh))
  (Class|PrimitiveComponent|SetPhysMaterialOverride _staticmesh (Variables|Default|GetPhysMaterial))
  (Rendering|Material|SetMaterial _staticmesh 0 (Variables|Default|GetMaterial)))