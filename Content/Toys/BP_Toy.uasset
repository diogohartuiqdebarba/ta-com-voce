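; BP_Toy is a toy actor with a configurable static mesh that briefly slows any Character that hits it.
; The construction script applies the Mesh and PhysMaterial variables to the StaticMesh component.
; On Hit, it prints a debug string and lowers the Character's MaxWalkSpeed, then after a short delay sets a fixed higher speed rather than restoring the previous value.
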(event Collision|EventHit
  (params (MyComp :type Primitive%20Component%20Object%20Reference) (Other :type Actor%20Object%20Reference) (OtherComp :type Primitive%20Component%20Object%20Reference) (bSelfMoved :type Boolean) (HitLocation :type Vector :default "0, 0, 0") (HitNormal :type Vector :default "0, 0, 0") (NormalImpulse :type Vector :default "0, 0, 0") (Hit :type Hit%20Result%20Structure%20%28by%20ref%29))
  (Development|PrintString "Hit Toy!" true true "(R=0.961351,G=1.000000,B=0.000000,A=1.000000)")
  (bind _ascharacter (Utilities|Casting|CastToCharacter Other))
  (Variables|/Script/Engine.CharacterMovementComponent|SetMaxWalkSpeed (Variables|/Script/Engine.Character|GetCharacterMovement _ascharacter) 3e+02)
  (Utilities|FlowControl|Delay 0.6)
  (Variables|/Script/Engine.CharacterMovementComponent|SetMaxWalkSpeed (Variables|/Script/Engine.Character|GetCharacterMovement _ascharacter) 5e+02))

(fn ConstructionScript
  (bind _staticmesh (Variables|Default|GetStaticMesh))
  (Components|StaticMesh|SetStaticMesh _staticmesh (Variables|Default|GetMesh))
  (Class|PrimitiveComponent|SetPhysMaterialOverride _staticmesh (Variables|Default|GetPhysMaterial)))