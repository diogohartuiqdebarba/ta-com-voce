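; Game manager for a tag minigame, started with Enter, that spawns the characters and picks a random "It".
; It possesses a random player character and recursively spawns NPCs, drawing from a shrinking class pool to avoid duplicate characters.
; The SetItActor dispatcher announces tag changes to ChangeIt, which swaps the It/NotIt music and HUD color.
; A DoOnce delay loop counts down on the widget before tagging is free again.
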(event Custom|ChangeIt
  (params (It :type Actor%20Object%20Reference) (TagFree :type Boolean))
  (bind _bpc_tagscorewidget (Variables|Default|GetBPC_TagScoreWidget))
  (bind _tagscorewidget (Variables|/Game/TagSystem/BPC_TagScoreWidget.BPC_TagScoreWidget_C|GetTagScoreWidget _bpc_tagscorewidget))
  ;[1 1 1] Set Can Tag Again Regressive
  (Development|PrintString "BP_Player: Change It Event!" true true "(R=1.000000,G=0.959391,B=0.000000,A=1.000000)")
  (if (not TagFree)
    (Utilities|Casting|CastToBP_Player It
      (:then
        (Components|Activation|SetActive (Variables|Default|GetItMusic) true false)
        (Components|Activation|SetActive (Variables|Default|GetNotItMusic) false false)
        (Default|SetTagColor _tagscorewidget true))
      (:CastFailed
        (Components|Activation|SetActive (Variables|Default|GetItMusic) false false)
        (Components|Activation|SetActive (Variables|Default|GetNotItMusic) true false)
        (Default|SetTagColor _tagscorewidget false)))
    (Utilities|FlowControl|DoOnce false :!label _label
      (:Completed
        (bind _cantagagaincount (Default|SetCanTagAgainRegressive (Variables|/Game/TagSystem/BPC_TagScoreWidget.BPC_TagScoreWidget_C|GetTagScoreWidget (Variables|Default|GetBPC_TagScoreWidget)) (Variables|Default|GetTimesToResetTagFree) :!label _label_2))
        (Utilities|FlowControl|Delay 1.0)
        (if (> _cantagagaincount 0)
          (goto _label_2)
          (else
            (Variables|Default|SetTagFree true)
            (goto _label Reset)))))))

(event EventBeginPlay
  (Input|EnableInput (Game|GetPlayerController 0))
  (Default|ShowStartGameText (Variables|/Game/TagSystem/BPC_TagScoreWidget.BPC_TagScoreWidget_C|GetTagScoreWidget (Variables|Default|GetBPC_TagScoreWidget)))
  (Utilities|FlowControl|Sequence
    (:then_0
      (bind _returnvalue (Audio|SpawnSound2D "/Game/Audio/GameMusics/it-music.it-music" 1.0 1.0 0.0 0 false false))
      (bind _output_get (Variables|Default|SetItMusic _returnvalue))
      (Components|Activation|SetActive _output_get false false))
    (:then_1
      (bind _returnvalue_2 (Audio|SpawnSound2D "/Game/Audio/GameMusics/not-it-music.not-it-music" 1.0 1.0 0.0 0 false false))
      (bind _output_get_2 (Variables|Default|SetNotItMusic _returnvalue_2))
      (Components|Activation|SetActive _output_get_2 true false)
      ;[1 1 1] Set Can Tag Again Regressive
      (EventDispatchers|BindEventtoSetItActor (delegate Custom|ChangeIt)))))

(event Input|KeyboardEvents|Enter
  (params (Key :type Key%20Structure :default "None"))
  (bind _bpc_tagscorewidget (Variables|Default|GetBPC_TagScoreWidget))
  (bind _tagscorewidget (Variables|/Game/TagSystem/BPC_TagScoreWidget.BPC_TagScoreWidget_C|GetTagScoreWidget _bpc_tagscorewidget))
  (:Pressed
    (Development|PrintString "Start Tag System." true true "(R=0.114219,G=1.000000,B=0.015114,A=1.000000)")
    (Audio|PlaySound2D "/Game/Audio/UI/start-game.start-game" 0.84 1.0 0.0 0 0)
    (bind _success (CallFunction|SpawnPlayer))
    (if _success
      (bind _success_2 (CallFunction|SpawnNPCs))
      (if _success_2
        (bind _playerisit (CallFunction|GetRandomIt))
        (Default|SetTagColor _tagscorewidget _playerisit)
        (Default|HideStartGameText _tagscorewidget)
        (Variables|Default|SetCanPlayersMove true)
        (else
          (Development|PrintString "Spawn NPCs Error!" true true "(R=1.000000,G=0.000000,B=0.000000,A=1.000000)")))
      (else
        (Development|PrintString "Spawn Player Error!" true true "(R=1.000000,G=0.000000,B=0.000000,A=1.000000)")))))

(fn ConstructionScript)

(fn GetRandomIt
  (bind _outactors (Actor|GetAllActorsOfClass "/Game/Characters/Blueprints/BP_BaseCharacter.BP_BaseCharacter_C"))
  (bind _output_get (Variables|Default|SetPlayers _outactors))
  (bind _output_get_2 (Variables|Default|SetIt (.OutItem (Utilities|Array|Random _output_get))))
  (Default|CallSetItActor _output_get_2 true)
  (Development|PrintString "Call Set It Actor!")
  (bind _asbp_base_character (Utilities|Casting|CastToBP_BaseCharacter _output_get_2))
  (Default|ShowItTagWidget _asbp_base_character)
  (Utilities|Casting|CastToBP_Player _output_get_2)
  (if true
    (return true)
    (else
      (return false))))

(fn SetIt
  (params (It :type Actor%20Object%20Reference))
  (bind _output_get (Variables|Default|SetIt It))
  (Default|CallSetItActor _output_get false)
  (Development|PrintString "BP_TagSystem: Call Set It Actor Event!" true true "(R=0.991526,G=1.000000,B=0.167918,A=1.000000)"))

(fn SpawnNPCs
  (bind _transformsnpc (Variables|Default|GetTransformsNPC))
  (bind _outitem (Utilities|Array|Random _transformsnpc))
  (if (>= (Variables|Default|GetCountNPCs) (LocalVariables|GetMaxNPCs))
    (return true)
    (else
      (bind _output_get (LocalVariables|SetClasseIndex (.OutItem (Utilities|Array|Random (Variables|Default|GetClassesCharacter)))))
      (Utilities|Array|RemoveItem (Variables|Default|GetClassesCharacter) _output_get)
      (Game|SpawnActorfromClass (Utilities|Select :Index (LocalVariables|GetClasseIndex) :Option%200 "/Game/Characters/Blueprints/NPCs/BP_NPC_Aika.BP_NPC_Aika_C" :Option%201 "/Game/Characters/Blueprints/NPCs/BP_NPC_Lili.BP_NPC_Lili_C" :Option%202 "/Game/Characters/Blueprints/NPCs/BP_NPC_Lucas.BP_NPC_Lucas_C" :Option%203 "/Game/Characters/Blueprints/NPCs/BP_NPC_Nina.BP_NPC_Nina_C" :Option%204 "/Game/Characters/Blueprints/NPCs/BP_NPC_Paulo.BP_NPC_Paulo_C") _outitem "Undefined" 0 0)
      (Variables|Default|SetCountNPCs (+ 1 (Variables|Default|GetCountNPCs)))
      (Utilities|Array|RemoveItem (Variables|Default|GetTransformsNPC) _outitem)
      (bind _success (CallFunction|SpawnNPCs))
      (return _success))))

(fn SpawnPlayer
  (bind _returnvalue (Game|GetPlayerCharacter 0))
  (bind _output_get (LocalVariables|SetClasseIndex (.OutItem (Utilities|Array|Random (Variables|Default|GetClassesCharacter)))))
  (Utilities|Array|RemoveItem (Variables|Default|GetClassesCharacter) _output_get)
  (bind _returnvalue_2 (Game|SpawnActorfromClass (Utilities|Select :Index (LocalVariables|GetClasseIndex) :Option%200 "/Game/Characters/Blueprints/Players/BP_Player_Aika.BP_Player_Aika_C" :Option%201 "/Game/Characters/Blueprints/Players/BP_Player_Lili.BP_Player_Lili_C" :Option%202 "/Game/Characters/Blueprints/Players/BP_Player_Lucas.BP_Player_Lucas_C" :Option%203 "/Game/Characters/Blueprints/Players/BP_Player_Nina.BP_Player_Nina_C" :Option%204 "/Game/Characters/Blueprints/Players/BP_Player_Paulo.BP_Player_Paulo_C") (Math|Transform|MakeTransform "-5.000000,-510.000000,212.000000" "0.000000,180.000000,0.000000") "Undefined" 0 0))
  (Variables|Default|SetDefaultPlayer _returnvalue)
  (Pawn|SpawnDefaultController (Variables|/Script/Engine.Actor|GetInstigator _returnvalue_2))
  (Pawn|Possess (Game|GetPlayerController (Variables|/Script/Engine.Pawn|GetPlayerState _returnvalue)) (Variables|/Script/Engine.Actor|GetInstigator _returnvalue_2))
  (Actor|DestroyActor (Variables|Default|GetDefaultPlayer))
  (return true))

(fn CheckEqualPlayers
  (params (Actor :type Actor%20Object%20Reference))
  (for _array_element (Variables|Default|GetPlayers)
    (if (== _array_element Actor)
      (return false)))
  (return false))